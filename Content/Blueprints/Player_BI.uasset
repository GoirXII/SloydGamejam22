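; Player_BI is a Blueprint Interface that exposes the player's stats and run state to other Blueprints without implementing any logic itself.
; Getter-style functions return XP progress, level, timer, kill count and living enemy count.
; Property functions return projectile and sword weapon stats, plus player health, speed, XP and arrow and sword unlock flags.
; DestroyOutOfRangeAI is the only call without outputs, named for culling distant AI.
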(fn `DestroyOutOfRangeAI`)

(fn `GetCurrentLevel`
  (returns (CurrentLevel :type Integer))
  (return 0))

(fn `GetXP`
  (returns (CurrentXP :type "Float (double-precision)") (MaxXP :type "Float (double-precision)"))
  (return 0.0 0.0))

(fn `PlayerProperties`
  (returns (MaxHealth :type "Float (double-precision)") (Current :type "Float (double-precision)") (Speed :type "Float (double-precision)") (XP :type "Float (double-precision)") (ArrowUnlock :type Boolean) (SwordUnlock :type Boolean))
  (return 0.0 0.0 0.0 0.0 false false))

(fn `ProjectileProperties`
  (returns (Cooldown :type "Float (double-precision)") (Amount :type Integer) (Pierce :type Integer) (Damage :type "Float (double-precision)"))
  (return 0.0 0 0 0.0))

(fn `SwordProperties`
  (returns (Cooldown :type "Float (double-precision)") (Speed :type "Float (double-precision)") (Damage :type "Float (double-precision)") (Lifespan :type "Float (double-precision)") (Spline :type "SplineComponent Object Reference"))
  (return 0.0 0.0 0.0 0.0 null))

(fn `UpdateEnemiesAlive`
  (returns (EnemiesAlive :type Integer))
  (return 0))

(fn `UpdateKillCount`
  (returns (KillCount :type Integer))
  (return 0))

(fn `UpdateTimer`
  (returns (Minutes :type Integer) (Seconds :type Integer))
  (return 0 0))