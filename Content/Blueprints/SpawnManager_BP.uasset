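; SpawnManager_BP is an enemy spawner that creates waves of randomly chosen enemy AI variants at its own location.
; On BeginPlay it binds SpawnEnemy to the respawn event of BP_TopDownGameMode.
; Each trigger spawns the current count of enemies, adjusting for collisions but always spawning.
; It then raises an increment and adds it to the count, so waves grow at an accelerating rate, and prints the new amount.
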(event `self.ReceiveBeginPlay`
  (bind _asbp_top_down_game_mode (cast `/Game/TopDown/Blueprints/BP_TopDownGameMode` (`GameplayStatics.GetGameMode`)))
  (add `/Game/TopDown/Blueprints/BP_TopDownGameMode.RespawnEnemy` _asbp_top_down_game_mode (delegate `SpawnEnemy`)))

(event `SpawnEnemy`
  ;[1 1 1] Spawn logic
  (for _ (range (`self.EnemiesSpawned`))
    (`|SpawnActorFromClass` (select `int` (`KismetMathLibrary.RandomInteger` 3) :`0` "/Game/AI/EnemyAI.EnemyAI_C" :`1` "/Game/AI/EnemyAI_02Green.EnemyAI_02Green_C" :`2` "/Game/AI/EnemyAI_03Yellow.EnemyAI_03Yellow_C" :`3` "/Game/AI/EnemyAI_05Red.EnemyAI_05Red_C" :!type "Actor Class Reference") (`KismetMathLibrary.MakeTransform` (`SceneComponent.K2_GetComponentLocation` (`self.DefaultSceneRoot`))) "AdjustIfPossibleButAlwaysSpawn" "OverrideRootScale" null null))
  (`/Engine/EditorBlueprintResources/StandardMacros.IncrementInt` (`self.IncrementSpawned`) ; increment amount of spawned enemies each time it loops
    (:`  `
      (bind _output_get (set `self.EnemiesSpawned` (+ (`self.EnemiesSpawned`) (`self.IncrementSpawned`))))
      (`KismetSystemLibrary.PrintString` (`KismetTextLibrary.Conv_TextToString` (`|FormatText` "Spawn amount: {X}" _output_get)) true true (struct :`G` 1.0 :`B` 0.056943 :`A` 1.0)))))

(fn `UserConstructionScript`)