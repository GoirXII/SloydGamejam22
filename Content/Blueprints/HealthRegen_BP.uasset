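; Health regeneration zone that heals a BP_TopDownCharacter entering its Box trigger.
; Begin overlap starts a Delay loop that adds 0.1 health and plays a sound at the character every two seconds, though the graph comment says one.
; The loop repeats while health is at most 1.0, so it can overshoot.
; End overlap clears InRange, but the loop never rechecks it, so healing continues outside the box.
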(event `self.Box.OnComponentBeginOverlap`
  (params (OverlappedComponent :type "PrimitiveComponent Object Reference") (OtherActor :type "Actor Object Reference") (OtherComp :type "PrimitiveComponent Object Reference") (OtherBodyIndex :type Integer) (bFromSweep :type Boolean) (SweepResult :type "HitResult Structure (by ref)"))
  ;[1 1 1] Health Regeneration - In Range? Then heal 0.1 every 1 sec
  (bind _asbp_top_down_character (cast `/Game/Character/BP_TopDownCharacter` OtherActor))
  (bind _output_get (set `self.InRange?` true))
  (if _output_get
    (bind _currenthealth (`/Game/Character/BP_TopDownCharacter.CurrentHealth` _asbp_top_down_character))
    (if (<= _currenthealth 1.0) :!label _label
      (set `/Game/Character/BP_TopDownCharacter.CurrentHealth` (+ _currenthealth 0.1) _asbp_top_down_character)
      (`GameplayStatics.PlaySoundAtLocation` "/Game/Sound/HealthRegenSound.HealthRegenSound" (`self.K2_GetActorLocation` _asbp_top_down_character) (struct) 1.0 1.0 0.0 null null null null)
      (`KismetSystemLibrary.Delay` 2.0)
      (goto _label))))

(event `self.Box.OnComponentEndOverlap`
  (params (OverlappedComponent :type "PrimitiveComponent Object Reference") (OtherActor :type "Actor Object Reference") (OtherComp :type "PrimitiveComponent Object Reference") (OtherBodyIndex :type Integer))
  ;[1 1 1] Health Regeneration - In Range? Then heal 0.1 every 1 sec
  (cast `/Game/Character/BP_TopDownCharacter` OtherActor)
  (set `self.InRange?` false))

(fn `UserConstructionScript`)