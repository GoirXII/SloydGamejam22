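; Arrow projectile actor that damages actors it overlaps and destroys itself after its lifespan expires.
; A sphere overlap with anything but the player character triggers damage, using Damage and Pierce values requested from the player character.
; With positive Pierce the arrow survives each hit, without decrementing the count; otherwise a DoOnce limits it to one hit before destruction.
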(event `self.ReceiveBeginPlay`
  ;[1 1 1] Projectile lifetime
  (`KismetSystemLibrary.Delay` (`self.ArrowLifespan`))
  (`self.K2_DestroyActor`))

(event `self.Sphere.OnComponentBeginOverlap`
  (params (OverlappedComponent :type "PrimitiveComponent Object Reference") (OtherActor :type "Actor Object Reference") (OtherComp :type "PrimitiveComponent Object Reference") (OtherBodyIndex :type Integer) (bFromSweep :type Boolean) (SweepResult :type "HitResult Structure (by ref)"))
  ;[1 1 1] Overlap events
  (if (not (== OtherActor (`GameplayStatics.GetPlayerCharacter` 0)))
    (set `self.DealDamage?` true)
    (`self.ApplyDamage`)))

(event `ApplyDamage`
  ;[1 1 1] Applies damage to overlapped actor
  (if (`self.DealDamage?`)
    (bind (_cooldown _amount _pierce _damage) (message `/Game/Blueprints/Player_BI.ProjectileProperties` (`GameplayStatics.GetPlayerCharacter` 0)))
    (if (> _pierce 0)
      (`GameplayStatics.ApplyDamage` (stale `self.Sphere.OnComponentBeginOverlap` OtherActor) _damage)
      (else
        (`/Engine/EditorBlueprintResources/StandardMacros.DoOnce` false
          (:`Completed`
            (`GameplayStatics.ApplyDamage` (stale `self.Sphere.OnComponentBeginOverlap` OtherActor) _damage)
            (`self.K2_DestroyActor`)))))))

(event `self.Sphere.OnComponentEndOverlap`
  (params (OverlappedComponent :type "PrimitiveComponent Object Reference") (OtherActor :type "Actor Object Reference") (OtherComp :type "PrimitiveComponent Object Reference") (OtherBodyIndex :type Integer))
  ;[1 1 1] Overlap events
  (set `self.DealDamage?` false))

(fn `UserConstructionScript`)