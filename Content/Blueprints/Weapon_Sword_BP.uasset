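; Sword weapon actor with a capsule collision, built to damage actors it overlaps.
; Its ApplyDamage event checks a DealDamage flag, then applies the damage value fetched from player 0's character through a SwordPropertiesMessage call.
; The BeginPlay and overlap events are empty.
; The lifespan-based destroy, flag toggling and player-excluding overlap check are disconnected, so nothing in this graph triggers damage.
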(event `self.ReceiveBeginPlay`
  ;[1 1 1] Projectile lifetime
)

(event `self.Capsule.OnComponentBeginOverlap`
  (params (OverlappedComponent :type "PrimitiveComponent Object Reference") (OtherActor :type "Actor Object Reference") (OtherComp :type "PrimitiveComponent Object Reference") (OtherBodyIndex :type Integer) (bFromSweep :type Boolean) (SweepResult :type "HitResult Structure (by ref)"))
  ;[1 1 1] Overlap events
)

(event `ApplyDamage`
  ;[1 1 1] Applies damage to overlapped actor
  (if (`self.DealDamage?`)
    (bind (_cooldown _amount _damage) (message `/Game/Blueprints/Player_BI.SwordProperties` (`GameplayStatics.GetPlayerCharacter` 0)))
    (`GameplayStatics.ApplyDamage` (stale `self.Capsule.OnComponentBeginOverlap` OtherActor) _damage)))

(event `self.Capsule.OnComponentEndOverlap`
  (params (OverlappedComponent :type "PrimitiveComponent Object Reference") (OtherActor :type "Actor Object Reference") (OtherComp :type "PrimitiveComponent Object Reference") (OtherBodyIndex :type Integer))
  ;[1 1 1] Overlap events
)

(fn `UserConstructionScript`)