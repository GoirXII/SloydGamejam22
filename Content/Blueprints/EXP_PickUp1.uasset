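; EXP_PickUp1 is a magnet-style pickup that, despite its EXP naming, gives health to the player.
; Entering the PickUpRange trigger starts a timeline after a short delay, moving the actor toward the player with VInterpTo plus the timeline track's value.
; Overlapping the Sphere calls GainHealth on BP_TopDownCharacter, prints a message and destroys the pickup.
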(event `self.PickUpRange.OnComponentBeginOverlap`
  (params (OverlappedComponent :type "PrimitiveComponent Object Reference") (OtherActor :type "Actor Object Reference") (OtherComp :type "PrimitiveComponent Object Reference") (OtherBodyIndex :type Integer) (bFromSweep :type Boolean) (SweepResult :type "HitResult Structure (by ref)"))
  ;[1 1 1] EXP is dragged to you
  (if (== OtherActor (`GameplayStatics.GetPlayerCharacter` 0))
    (`KismetSystemLibrary.Delay` 0.2)
    (bind (_direction _newtrack_1) (`Timeline|Timeline_0`)
      (:`Update`
        (`self.K2_SetActorLocation` (+ _newtrack_1 (`KismetMathLibrary.VInterpTo` (.location (`self.GetTransform`)) (`self.K2_GetActorLocation` (`GameplayStatics.GetPlayerCharacter` 0)) (`GameplayStatics.GetWorldDeltaSeconds`) 8.0)))))))

(event `self.Sphere.OnComponentBeginOverlap`
  (params (OverlappedComponent :type "PrimitiveComponent Object Reference") (OtherActor :type "Actor Object Reference") (OtherComp :type "PrimitiveComponent Object Reference") (OtherBodyIndex :type Integer) (bFromSweep :type Boolean) (SweepResult :type "HitResult Structure (by ref)"))
  (bind _returnvalue (`GameplayStatics.GetPlayerCharacter` 0))
  ;[1 1 1] EXP is destroyed
  (if (== OtherActor _returnvalue)
    (bind _asbp_top_down_character (cast `/Game/Character/BP_TopDownCharacter` _returnvalue))
    (`/Game/Character/BP_TopDownCharacter.Gain Health` _asbp_top_down_character)
    (`KismetSystemLibrary.PrintString` "Give Health")
    (`self.K2_DestroyActor` self)))

(fn `UserConstructionScript`)