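; Boss spawner actor that spawns escalating batches of EnemyAI_04Orange enemies at its root location.
; On BeginPlay it binds its spawn event to the SpawnBoss dispatcher on BP_TopDownGameMode.
; Each trigger spawns the current count, adjusting for collisions but always spawning.
; It then increments the step and adds it to the count, so waves grow faster than linearly, and prints the new amount.
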(event `self.ReceiveBeginPlay`
  (bind _asbp_top_down_game_mode (cast `/Game/TopDown/Blueprints/BP_TopDownGameMode` (`GameplayStatics.GetGameMode`)))
  (add `/Game/TopDown/Blueprints/BP_TopDownGameMode.SpawnBoss` _asbp_top_down_game_mode (delegate `SpawnEnemyBoss`)))

(event `SpawnEnemyBoss`
  ;[1 1 1] Spawn logic
  (for _ (range (`self.EnemiesSpawned`))
    (`|SpawnActorFromClass` "/Game/AI/EnemyAI_04Orange.EnemyAI_04Orange_C" (`KismetMathLibrary.MakeTransform` (`SceneComponent.K2_GetComponentLocation` (`self.DefaultSceneRoot`))) "AdjustIfPossibleButAlwaysSpawn" "OverrideRootScale" null null))
  (`/Engine/EditorBlueprintResources/StandardMacros.IncrementInt` (`self.IncrementSpawned`) ; increment amount of spawned enemies each time it loops
    (:`  `
      (bind _output_get (set `self.EnemiesSpawned` (+ (`self.EnemiesSpawned`) (`self.IncrementSpawned`))))
      (`KismetSystemLibrary.PrintString` (`KismetTextLibrary.Conv_TextToString` (`|FormatText` "Spawn amount: {X}" _output_get)) true true (struct :`G` 1.0 :`B` 0.056943 :`A` 1.0)))))

(fn `UserConstructionScript`)